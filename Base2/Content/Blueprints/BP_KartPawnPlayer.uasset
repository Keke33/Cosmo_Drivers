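; BP_KartPawnPlayer is the player-controlled kart pawn, translating player input into kart driving commands.
; The Move Forward and Move Right axes feed throttle and steering setters, and the E key toggles debug mode.
; The graph holds only this input wiring: BeginPlay, overlap and Tick are disabled stubs, and the construction script just calls its parent.
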(event `InputAxis|Move Forward`
  (params (AxisValue :type "Float (single-precision)"))
  (`self.Set Throttle Input` AxisValue))

(event `InputAxis|Move Right`
  (params (AxisValue :type "Float (single-precision)"))
  (`self.Set Steering Input` AxisValue))

(event `Key|E`
  (params (Key :type "Key Structure"))
  (:`Pressed`
    (`self.Toggle Debug Mode`)))

(fn `UserConstructionScript`
  (`parent.UserConstructionScript`))